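; BP_WM_Pawn is the WeatherMachine pawn, providing orbit-style view rotation through a spring arm.
; Each Tick adds input axis values to the arm's yaw and pitch, clamping pitch and holding roll at zero.
; Left mouse press and release set IsDragging, but the branch that reads it is unconnected, so rotation runs whether or not the button is held.
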(event `self.ReceiveTick`
  (params (DeltaSeconds :type "Float (single-precision)"))
  (bind _springarm (`self.SpringArm`))
  (bind (_relativerotation_roll _relativerotation_pitch _relativerotation_yaw) (`KismetMathLibrary.BreakRotator` (`SceneComponent.RelativeRotation` _springarm)))
  (`SceneComponent.K2_SetRelativeRotation` _springarm (`KismetMathLibrary.MakeRotator` 0.0 (`KismetMathLibrary.FClamp` (+ _relativerotation_pitch (`self.GetInputAxisKeyValue`)) -80.0 60.0) (+ (`self.GetInputAxisKeyValue`) _relativerotation_yaw)) false false))

(event `Key|LeftMouseButton`
  (params (Key :type "Key Structure"))
  (:`Pressed`
    (set `self.IsDragging` true))
  (:`Released`
    (set `self.IsDragging` false)))

(fn `UserConstructionScript`)
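; BP_WeatherMachine displays live or historic weather data in the level and on a WBP_UI HUD.
; Tick eases displayed sun and wind toward TargetWeather, snapping large sun jumps, and drives MPC_Weather through light curves and a tree-scaled wind range.
; Right click toggles live/historic and the wheel steps history IDs, using functions defined outside this graph.
; JSON file-exchange helpers remain, but the event graph never calls them.
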(event `self.ReceiveBeginPlay`
  ; New Implementation
  ;; Begin
  (`|ExecutionSequence`
    (:`then_0`
      (`self.SetupUI`) ; Call this first or it will crash when any on repnotify variable changes
    )))

(event `self.OnTargetWeatherChanged`
  (params (NewTargetWeather :type "WeatherPacket Structure (by ref)"))
  ; New Implementation
  ;; Display
  (`self.UpdateHudWithTargetStruct` NewTargetWeather))

(event `self.OnHistoricIdRequest`
  (params (NewHistoricIdRequested :type Integer))
  ; New Implementation
  ;; Display
  (bind _as_wbp_ui (`self.As WBP UI`)
    (:`then`
      (`/Game/WeatherMachine/WBP_UI.SetTextFromMap` _as_wbp_ui "NewEnumerator2" (`KismetTextLibrary.Conv_IntToText` NewHistoricIdRequested)))
    (:`else`)))

(event `self.OnToggleIsLive`
  (params (bIsLiveState :type Boolean))
  ; New Implementation
  ;; Display
  (bind _as_wbp_ui (`self.As WBP UI`)
    (:`then`
      (if bIsLiveState
        (`/Game/WeatherMachine/WBP_UI.SetTextFromMap` _as_wbp_ui "NewEnumerator5" "Live")
        (else
          (`/Game/WeatherMachine/WBP_UI.SetTextFromMap` _as_wbp_ui "NewEnumerator5" "Historic"))))
    (:`else`)))

(event `self.ReceiveTick`
  (params (DeltaSeconds :type "Float (single-precision)"))
  (bind _returnvalue (`KismetMathLibrary.FInterpTo` (`.WindSpeed` (break `WeatherPacket` (`self.DisplayWeather`))) (`.WindSpeed` (break `WeatherPacket` (`self.TargetWeather`))) DeltaSeconds 1.0))
  (bind _returnvalue_2 (`KismetMathLibrary.FInterpTo` (`.SunAlpha` (break `WeatherPacket` (`self.DisplayWeather`))) (`.SunAlpha` (break `WeatherPacket` (`self.TargetWeather`))) DeltaSeconds 1.0))
  ; New Implementation
  ;; Tick
  (`|ExecutionSequence`
    (:`then_0`
      ;;; Interp To Display
      ;;;; Sun Alpha
      (if (> (`KismetMathLibrary.Abs` (- (`.SunAlpha` (break `WeatherPacket` (`self.DisplayWeather`))) (`.SunAlpha` (break `WeatherPacket` (`self.TargetWeather`))))) 0.5)
        (setmembers `WeatherPacket` :`StructRef` (`self.DisplayWeather`) :`SunAlpha` (`.SunAlpha` (break `WeatherPacket` (`self.TargetWeather`))))
        (`KismetMaterialLibrary.SetScalarParameterValue` "/Game/WeatherMachine/MPC_Weather.MPC_Weather" "LightAmount" (`CurveFloat.GetFloatValue` (`self.SunLightCurve`) (`.SunAlpha` (break `WeatherPacket` (`self.DisplayWeather`)))))
        (`KismetMaterialLibrary.SetVectorParameterValue` "/Game/WeatherMachine/MPC_Weather.MPC_Weather" "LightColor" (`CurveLinearColor.GetLinearColorValue` (`self.SunColorCurve`) (`.SunAlpha` (break `WeatherPacket` (`self.DisplayWeather`)))))
        (else
          (setmembers `WeatherPacket` :`StructRef` (`self.DisplayWeather`) :`SunAlpha` _returnvalue_2)
          (`KismetMaterialLibrary.SetScalarParameterValue` "/Game/WeatherMachine/MPC_Weather.MPC_Weather" "LightAmount" (`CurveFloat.GetFloatValue` (`self.SunLightCurve`) _returnvalue_2))
          (`KismetMaterialLibrary.SetVectorParameterValue` "/Game/WeatherMachine/MPC_Weather.MPC_Weather" "LightColor" (`CurveLinearColor.GetLinearColorValue` (`self.SunColorCurve`) _returnvalue_2)))))
    (:`then_2`
      ;;;; WindSpeed
      (setmembers `WeatherPacket` :`StructRef` (`self.DisplayWeather`) :`WindSpeed` _returnvalue)
      (`KismetMaterialLibrary.SetScalarParameterValue` "/Game/WeatherMachine/MPC_Weather.MPC_Weather" "WindSpeed" (`KismetMathLibrary.MapRangeClamped` _returnvalue 0.0 50.0 0.0 0.7)))))

(event `Key|RightMouseButton` :paused true
  (params (Key :type "Key Structure"))
  ; New Implementation
  ;; History Interaction
  ;;; Toggle State
  (:`Released`
    (`self.SetLiveState` (not (`self.bIsLive`)))))

(event `Key|MouseScrollUp`
  (params (Key :type "Key Structure"))
  ; New Implementation
  ;; History Interaction
  ;;; Set Desired ID
  (:`Pressed`
    (`self.ShiftHistoricId` 1)))

(event `Key|MouseScrollDown`
  (params (Key :type "Key Structure"))
  ; New Implementation
  ;; History Interaction
  ;;; Set Desired ID
  (:`Pressed`
    (`self.ShiftHistoricId` -1)))

(fn `FindEnvironmentalActor`
  (params (ActorClassToFind :type "Actor Class Reference") (RelevantTag :type Name))
  (returns (ActorClassFound :type "Actor Object Reference"))
  (locals (Class :type "Actor Class Reference") (Tag :type Name) (ActorToSet :type "Actor Object Reference"))
  (`|ExecutionSequence`
    (:`then_0`
      (set `local.Class` ActorClassToFind)
      (set `local.Tag` RelevantTag))
    (:`then_1`
      (bind _outactors (`GameplayStatics.GetAllActorsOfClassWithTag` (`local.Class`) (`local.Tag`)))
      (`|ExecutionSequence`
        (:`then_0`
          ; If there are multiple actors with the tag print a warning
          (if (> (`KismetArrayLibrary.Array_Length` _outactors) 1)
            (`self.PrintLogWarning` "FindEnvironmentalActor" (`KismetStringLibrary.Concat_StrStr` "Found multipue Actors of class " (`KismetSystemLibrary.GetClassDisplayName` (`local.Class`)) " with tag" (`KismetStringLibrary.Conv_NameToString` (`local.Tag`)) " the first one found will be used"))))
        (:`then_1`
          ; was a valid actor found with the tag
          (bind _output_get (set `local.ActorToSet` (`|GetArrayItem` _outactors)))
          (if (`KismetSystemLibrary.IsValid` _output_get)
            ; Print the actor found and output it to be set
            (`self.PrintLog` "FindEnvironmentalActor" (`KismetStringLibrary.Concat_StrStr` "Found Actor " (`KismetSystemLibrary.GetDisplayName` (`local.ActorToSet`)) " with tag" (`KismetStringLibrary.Conv_NameToString` (`local.Tag`))))
            (return (`local.ActorToSet`))
            (else
              (bind _outactors_2 (`GameplayStatics.GetAllActorsOfClass` (`local.Class`)))
              (`|ExecutionSequence`
                (:`then_0`
                  ; If there are multiple Actors of the same class print a warning
                  (if (> (`KismetArrayLibrary.Array_Length` _outactors_2) 1)
                    (`self.PrintLogWarning` "FindEnvironmentalActor" (`KismetStringLibrary.Concat_StrStr` "Found multipue Actors of class " (`KismetSystemLibrary.GetClassDisplayName` (`local.Class`)) " use Tag" (`KismetStringLibrary.Conv_NameToString` (`local.Tag`)) "to set a specific Actor"))))
                (:`then_1`
                  (bind _output (`|GetArrayItem` _outactors_2))
                  (if (`KismetSystemLibrary.IsValid` _output)
                    (set `local.ActorToSet` _output)
                    ; Print the actor found and output it to be set
                    (`self.PrintLog` "FindEnvironmentalActor" (`KismetStringLibrary.Concat_StrStr` "Found Actor " (`KismetSystemLibrary.GetDisplayName` (`local.ActorToSet`))))
                    (return (`local.ActorToSet`))
                    (else
                      ; No Valid Actor was Found
                      (`self.PrintError` "FindEnvironmentalActor" (`KismetStringLibrary.Concat_StrStr` "No Valid Actor of class " (`KismetSystemLibrary.GetClassDisplayName` (`local.Class`)) " was found with or without Tag " (`KismetStringLibrary.Conv_NameToString` (`local.Tag`))))
                      (return null))))))))))))

(fn `GetInterpSpeed`
  (params (UpdateIntervalSpeed :type "Float (double-precision)"))
  (returns (InterpSpeed :type "Float (double-precision)"))
  (return (/ (* UpdateIntervalSpeed 0.1) 1.0)))

(fn `HistoryRequest`
  (if (not (`self.HistoryLock`))
    (set `self.HistoryLock` true)
    (bind (_jsonout _filepathout _success) (`self.LoadJsonMakeIfNot` (`self.GetJsonFilePath` "unreal_control.json")))
    (if _success
      (`self.WriteToControlJson` _jsonout _filepathout)
      (else
        (`self.PrintError` "PauseState" "CouldNotAccessJson State.json")))))

(fn `LoadJsonMakeIfNot`
  (params (FilePath :type "FilePath Structure"))
  (returns (JsonOut :type "JsonObjectWrapper Structure") (FilePathOut :type "FilePath Structure") (Success :type Boolean))
  (locals (Json :type "JsonObjectWrapper Structure") (FilePathLocal :type "FilePath Structure"))
  (set `local.FilePathLocal` FilePath)
  (bind (_outjsonobject _returnvalue) (`JsonBlueprintFunctionLibrary.FromFile` FilePath))
  (if _returnvalue
    (set `local.Json` _outjsonobject)
    (else
      (bind _returnvalue_2 (`JsonBlueprintFunctionLibrary.ToFile` _outjsonobject (`local.FilePathLocal`)))
      (if _returnvalue_2
        (set `local.Json` _outjsonobject)
        (else
          (return (struct) (struct) false)))))
  (return (`local.Json`) (`local.FilePathLocal`) true))

(fn `OnRep_bBridgeConnected`
  (locals (TextToSet :type Text))
  (`|ExecutionSequence`
    (:`then_0`
      (if (`self.bSourceConnected`)
        (set `local.TextToSet` "Connected")
        (else
          (set `local.TextToSet` "Disconnected"))))
    (:`then_1`
      (bind _as_wbp_ui (`self.As WBP UI`)
        (:`then`
          (`/Game/WeatherMachine/WBP_UI.SetTextFromMap` _as_wbp_ui "NewEnumerator8" (`local.TextToSet`)))
        (:`else`)))))

(fn `OnRep_bSourceConnected`
  (locals (TextToSet :type Text))
  (`|ExecutionSequence`
    (:`then_0`
      (if (`self.bSourceConnected`)
        (set `local.TextToSet` "Connected")
        (else
          (set `local.TextToSet` "Disconnected"))))
    (:`then_1`
      (bind _as_wbp_ui (`self.As WBP UI`)
        (:`then`
          (`/Game/WeatherMachine/WBP_UI.SetTextFromMap` _as_wbp_ui "NewEnumerator0" (`local.TextToSet`)))
        (:`else`)))))

(fn `SetupControlJson`)

(fn `SetupUI`
  (bind _returnvalue (`|CreateWidget` "/Game/WeatherMachine/WBP_UI.WBP_UI_C"))
  (bind _output_get (set `self.As WBP UI` _returnvalue))
  (`UserWidget.AddToViewport` _output_get 0))

(fn `UpdateHudWithTargetStruct`
  (params (TargetWeatherPacket :type "WeatherPacket Structure"))
  (locals (TextToSet :type Text))
  (bind (_id _islive _sunalpha _timeiso _tempc _windspeed _cloudspercent _weatherstateid) (break `WeatherPacket` TargetWeatherPacket))
  (`|ExecutionSequence`
    (:`then_2`
      (bind _as_wbp_ui (`self.As WBP UI`)
        (:`then`
          (`/Game/WeatherMachine/WBP_UI.SetTextFromMap` _as_wbp_ui "NewEnumerator1" (`KismetTextLibrary.Conv_IntToText` _id)))
        (:`else`)))
    (:`then_3`
      (bind _as_wbp_ui_2 (`self.As WBP UI`)
        (:`then`
          (`/Game/WeatherMachine/WBP_UI.SetTextFromMap` _as_wbp_ui_2 "NewEnumerator3" (`KismetTextLibrary.Conv_IntToText` (`self.HighestId`))))
        (:`else`)))
    (:`then_4`
      (bind _as_wbp_ui_3 (`self.As WBP UI`)
        (:`then`
          (`/Game/WeatherMachine/WBP_UI.SetTextFromMap` _as_wbp_ui_3 "NewEnumerator4" (`KismetTextLibrary.Conv_IntToText` _weatherstateid)))
        (:`else`)))
    (:`then_5`
      (bind _as_wbp_ui_4 (`self.As WBP UI`)
        (:`then`
          (`/Game/WeatherMachine/WBP_UI.SetTextFromMap` _as_wbp_ui_4 "NewEnumerator6" (`KismetTextLibrary.Conv_StringToText` _timeiso)))
        (:`else`)))))

(fn `UpdateWeatherStructs`
  (params (TempWeatherStruct :type "/Game/WeatherMachine/Data/Struct_Weather Structure"))
  (locals (TempWeather :type "/Game/WeatherMachine/Data/Struct_Weather Structure"))
  (bind _as_wbp_ui (`self.As WBP UI`))
  (set `local.TempWeather` TempWeatherStruct)
  ; Is the file relevant to our request
  (if (== (`.IsLive_29_225AB62D4D0B2B8ADF4AEABA2C2B961B` (break `/Game/WeatherMachine/Data/Struct_Weather` (`local.TempWeather`))) (`self.bLive`))
    (`|ExecutionSequence`
      (:`then_1`
        (bind _output_get (set `self.NewWeatherData` (`local.TempWeather`)))
        (bind (_idmax _idcurrent _timestamp _sunalpha _windspeed _updatespeed _weatherstate _time_iso) (break `/Game/WeatherMachine/Data/Struct_Weather` _output_get))
        (`/Game/WeatherMachine/WBP_UI.SetTextFromMap` _as_wbp_ui "NewEnumerator6" (`KismetTextLibrary.Conv_StringToText` _time_iso))
        (`/Game/WeatherMachine/WBP_UI.SetTextFromMap` _as_wbp_ui "NewEnumerator4" (`KismetTextLibrary.Conv_IntToText` _weatherstate))
        (if (`self.bLive`)
          (bind _output_get_2 (set `self.MaxID` _idmax))
          (bind _output_get_3 (set `self.CurrentHistoricID` _output_get_2))
          (set `self.DesiredID` _output_get_3)
          (else
            (set `self.CurrentHistoricID` _idcurrent)))))))

(fn `UserConstructionScript`)

(fn `WeatherJsonToStruct`
  (params (Json :type "JsonObjectWrapper Structure"))
  (returns (TempWeather :type "/Game/WeatherMachine/Data/Struct_Weather Structure"))
  (locals (JsonLocal :type "JsonObjectWrapper Structure") (InterpSpeed :type "Float (double-precision)") (WeatherState :type Integer) (WindSpeed :type "Float (double-precision)") (SunAlpha :type "Float (double-precision)") (TimestampUnix :type Integer) (TimeIso :type String) (Current_ID :type Integer) (Max_ID :type Integer) (TempWeatherStruct :type "/Game/WeatherMachine/Data/Struct_Weather Structure") (LocalIsLive :type Boolean :default false))
  ; Handoff the json to a struct
  (set `local.JsonLocal` Json)
  (`|ExecutionSequence`
    (:`then_0`
      (`|ExecutionSequence`
        (:`then_0`
          (bind _outvalue (`|GetJsonField` (`local.JsonLocal`) "sun_alpha"))
          (set `local.SunAlpha` _outvalue))
        (:`then_1`
          (bind _outvalue_2 (`|GetJsonField` (`local.JsonLocal`) "wind_speed"))
          (set `local.WindSpeed` _outvalue_2))
        (:`then_2`
          (bind _outvalue_3 (`|GetJsonField` (`local.JsonLocal`) "weather_state_id"))
          (set `local.WeatherState` _outvalue_3))
        (:`then_3`
          (`|ExecutionSequence`
            (:`then_0`
              (bind _outvalue_4 (`|GetJsonField` (`local.JsonLocal`) "update_interval_time"))
              (bind _interpspeed (`self.GetInterpSpeed` _outvalue_4))
              (set `local.InterpSpeed` _interpspeed))
            (:`then_1`
              (bind _outvalue_5 (`|GetJsonField` (`local.JsonLocal`) "timestamp_unix"))
              (set `local.TimestampUnix` _outvalue_5))
            (:`then_2`
              (bind _outvalue_6 (`|GetJsonField` (`local.JsonLocal`) "current_id"))
              (set `local.Current_ID` _outvalue_6))
            (:`then_3`
              (`|ExecutionSequence`
                (:`then_0`
                  (bind _outvalue_7 (`|GetJsonField` (`local.JsonLocal`) "max_id"))
                  (set `local.Max_ID` _outvalue_7))
                (:`then_1`
                  (bind _outvalue_8 (`|GetJsonField` (`local.JsonLocal`) "is_live"))
                  (set `local.LocalIsLive` _outvalue_8))
                (:`then_2`
                  (bind _outvalue_9 (`|GetJsonField` (`local.JsonLocal`) "time_iso"))
                  (set `local.TimeIso` _outvalue_9))))))))
    (:`then_1`
      (return (make `/Game/WeatherMachine/Data/Struct_Weather` (`local.Max_ID`) (`local.Current_ID`) 0 (`local.SunAlpha`) (`local.WindSpeed`) (`local.InterpSpeed`) (`local.WeatherState`) (`local.TimeIso`) (`local.LocalIsLive`))))))

(fn `WriteToControlJson`
  (params (Json :type "JsonObjectWrapper Structure") (File :type "FilePath Structure"))
  (locals (JsonLocal :type "JsonObjectWrapper Structure") (Filepath :type "FilePath Structure"))
  (set `local.JsonLocal` Json)
  (set `local.Filepath` File)
  (`|SetJsonField` (`local.JsonLocal`) "is_live" (`self.bLive`))
  (`|SetJsonField` (`local.JsonLocal`) "desired_id" (`self.DesiredID`))
  (`JsonBlueprintFunctionLibrary.ToFile` (`local.JsonLocal`) (`local.Filepath`)))